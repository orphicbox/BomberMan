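; Map generator that builds a square Bomberman-style grid arena centred on the world origin at BeginPlay.
; Each cell index becomes a grid position, with indestructible walls where both coordinates are odd.
; Other cells get destructible walls by random chance, except the first and last, kept clear as player spawn points.
; Helper functions place the four boundary walls and move the blue and red players to opposite corners.
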(event `self.ReceiveBeginPlay`
  (bind _worlddimension (`self.WorldDimension`))
  (bind _returnvalue (/ (* (* (`self.WorldDimension`) (`self.WallBlockSize`)) -1.0) 2.0))
  (`|ExecutionSequence`
    (:`then_1`
      ;[1 1 1] Determine First Wall Block Location
      (set `self.FirstBlockPosition` (`KismetMathLibrary.MakeVector` _returnvalue _returnvalue 70.0)))
    (:`then_2`
      (bind _output_get (set `self.LastBlockNo` (- (* _worlddimension _worlddimension) 1)))
      (for _index (range (+ _output_get 1))
        ;[1 1 1] Create World Matrix
        (bind _output_get_2 (set `self.CurrentIndex` _index))
        (bind (_matrix_x _matrix_y _location_x _location_y) (`self.GetMatrixIndex` _output_get_2))
        (set `self.Matrix_X` _matrix_x)
        (set `self.Matrix_Y` _matrix_y)
        (bind _transform (`self.GetCellTransform` _location_x _location_y))
        (set `self.CellTransform` _transform)
        (bind _result (`self.IsStaticWallPlace` (`self.Matrix_X`) (`self.Matrix_Y`))) ; Should place static wall here ?
        (if _result
          ;[1 1 1] Spawn Indestructible Walls
          (`|SpawnActorFromClass` "/Game/Blueprints/IndestructibleWall_BP.IndestructibleWall_BP_C" (`self.CellTransform`) "Undefined" "OverrideRootScale" null null)
          (else
            ;[1 1 1] Is player spawn point?
            (if (not (or (== (`self.CurrentIndex`) 0) (== (`self.CurrentIndex`) (`self.LastBlockNo`))))
              ;[1 1 1] Check Spawn Destructible Wall Chance
              (if (< (`KismetMathLibrary.RandomFloat`) (`self.DestructibleWallChance`))
                ;[1 1 1] Spawn Destructible Wall
                (`|SpawnActorFromClass` "/Game/Blueprints/DestructibleWall_BP.DestructibleWall_BP_C" (`self.CellTransform`) "Undefined" "OverrideRootScale" null null)))))))))

(fn `GetCellTransform`
  (params (X :type "Float (double-precision)") (Y :type "Float (double-precision)"))
  (returns (Transform :type "Transform Structure"))
  (return (`KismetMathLibrary.Conv_VectorToTransform` (+ (`KismetMathLibrary.MakeVector` X Y) (`self.FirstBlockPosition`)))))

(fn `GetMatrixIndex`
  (params (Index :type Integer))
  (returns (Matrix_X :type Integer) (Matrix_Y :type Integer) (Location_X :type "Float (double-precision)") (Location_Y :type "Float (double-precision)"))
  (bind _worlddimension (`self.WorldDimension`))
  (bind _wallblocksize (`self.WallBlockSize`))
  (bind _returnvalue (/ Index _worlddimension))
  (bind _returnvalue_2 (mod Index _worlddimension))
  (return _returnvalue_2 _returnvalue (* _returnvalue_2 _wallblocksize) (* _returnvalue _wallblocksize)))

(fn `GetWorldHalfSize`
  (returns (ReturnValue :type "Float (double-precision)"))
  (return (/ (* (`self.WorldDimension`) (`self.WallBlockSize`)) 2.0)))

(fn `IsStaticWallPlace`
  (params (X :type Integer) (Y :type Integer))
  (returns (Result :type Boolean))
  (return (and (!= (mod X 2) 0) (!= (mod Y 2) 0))))

(fn `SetMapBoundries`
  (params (LeftWall :type "Actor Object Reference") (RightWall :type "Actor Object Reference") (NorthWall :type "Actor Object Reference") (SouthWall :type "Actor Object Reference"))
  (locals (WorldHSize :type "Float (double-precision)" :default 0.0))
  (bind _returnvalue (`self.GetWorldHalfSize`))
  (set `local.WorldHSize` _returnvalue)
  (`|ExecutionSequence`
    (:`then_0`
      (`self.K2_SetActorLocation` LeftWall (`KismetMathLibrary.MakeVector` 0.0 (* (+ (`local.WorldHSize`) (/ (`self.WallBlockSize`) 2.0)) -1.0)) false true))
    (:`then_1`
      (`self.K2_SetActorLocation` RightWall (`KismetMathLibrary.MakeVector` 0.0 (- (`local.WorldHSize`) (/ (`self.WallBlockSize`) 2.0))) false false))
    (:`then_2`
      (`self.K2_SetActorLocation` NorthWall (`KismetMathLibrary.MakeVector` (- (`local.WorldHSize`) (/ (`self.WallBlockSize`) 2.0))) false true))
    (:`then_3`
      (`self.K2_SetActorLocation` SouthWall (`KismetMathLibrary.MakeVector` (* (+ (`local.WorldHSize`) (/ (`self.WallBlockSize`) 2.0)) -1.0)) false true))))

(fn `SetPlayersSpawnPoints`
  (params (PlayerBlue :type "Actor Object Reference") (PlayerRed :type "Actor Object Reference"))
  (locals (WorldHSize :type "Float (double-precision)" :default 0.0))
  (bind _returnvalue (- (`local.WorldHSize`) (`self.WallBlockSize`)))
  (bind _returnvalue_2 (* (`local.WorldHSize`) -1.0))
  (bind _returnvalue_3 (`self.GetWorldHalfSize`))
  (set `local.WorldHSize` _returnvalue_3)
  (`|ExecutionSequence`
    (:`then_0`
      (`self.K2_SetActorLocation` PlayerBlue (`KismetMathLibrary.MakeVector` _returnvalue_2 _returnvalue_2 60.0) false true))
    (:`then_1`
      (`self.K2_SetActorLocation` PlayerRed (`KismetMathLibrary.MakeVector` _returnvalue _returnvalue 60.0) false false))))

(fn `UserConstructionScript`)