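; Movement helper functions for BomberMan that shift a target actor along the world X axis (forward) or Y axis (right).
; Each scales a direction input by speed and world delta seconds, then adds the offset to the actor's current location.
; The new location is set directly with sweep off, so the move itself does not stop at blocking geometry.
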(fn `BomberMan_MoveForward`
  (params (Direction :type "Float (double-precision)") (Target :type "Actor Object Reference") (Speed :type "Float (double-precision)"))
  (locals (Pspeed :type "Float (double-precision)"))
  (`Actor.K2_SetActorLocation` Target (+ (`KismetMathLibrary.MakeVector` (* Direction (* Speed (`GameplayStatics.GetWorldDeltaSeconds` null)))) (`Actor.K2_GetActorLocation` Target)) false false))

(fn `BomberMan_MoveRight`
  (params (Direction :type "Float (double-precision)" :default 0.0) (Target :type "Actor Object Reference") (Speed :type "Float (double-precision)"))
  (`Actor.K2_SetActorLocation` Target (+ (`KismetMathLibrary.MakeVector` 0.0 (* Direction (* Speed (`GameplayStatics.GetWorldDeltaSeconds` null)))) (`Actor.K2_GetActorLocation` Target)) false false))