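; Bomberman-style bomb actor that, after a fuse delay, explodes in a cross along the four horizontal world axes.
; Each arm line-traces for walls identified by first actor tag to set its length, then spawns a beam emitter to match.
; A multi-trace over that length gathers tagged players, items and destructible walls.
; After a short delay it destroys those victims and itself.
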(event `self.ReceiveBeginPlay`
  (`KismetSystemLibrary.Delay` (`self.ExplosionDelay`))
  (for _index (range 4)
    (bind _direction (`self.GetDirectionVector` _index))
    (bind _explosionlenght (`self.TraceObstacle` _direction))
    (`self.SpawnExplosionEmitter` _explosionlenght _index)
    (bind _actors (`self.TraceVictims` _direction _explosionlenght))
    (for _array_element _actors
      (`KismetArrayLibrary.Array_Add` (`self.VictimsArray`) _array_element)))
  (`KismetSystemLibrary.Delay` 0.5)
  ;[1 1 1] Destroy Victims
  (for _array_element_2 (`self.VictimsArray`)
    (`/Engine/EditorBlueprintResources/StandardMacros.IsValid` _array_element_2
      (:`Is Valid`
        (`self.K2_DestroyActor` _array_element_2))))
  ;[1 1 1] remove bomb
  (`self.K2_DestroyActor`))

(fn `GetDirectionVector`
  (params (Index :type Integer))
  (returns (Direction :type "Vector Structure"))
  (switch `int` Index
    (:`0`
      (return (1.0 0.0 0.0)))
    (:`1`
      (return (0.0 1.0 0.0)))
    (:`2`
      (return (-1.0 0.0 0.0)))
    (:`3`
      (return (0.0 -1.0 0.0)))))

(fn `IsBlockableObstacle`
  (params (Obstacle :type "Actor Object Reference"))
  (returns (Result :type Boolean))
  (bind _tags (`Actor.Tags` Obstacle))
  (if (`KismetArrayLibrary.Array_IsValidIndex` _tags)
    (set `self.HitActorTags` _tags)
    (return (or (== (`|GetArrayItem` (`self.HitActorTags`)) "IndestructibleWall") (== (`|GetArrayItem` (`self.HitActorTags`)) "DestructibleWall")))))

(fn `IsVictim`
  (params (Actor :type "Actor Object Reference"))
  (returns (Result :type Boolean))
  (bind _tags (`Actor.Tags` Actor))
  (bind _output (`|GetArrayItem` (`self.HitActorTags`)))
  (if (`KismetArrayLibrary.Array_IsValidIndex` _tags)
    (set `self.HitActorTags` _tags)
    (return (or (== _output "Speed_Item") (== _output "RemoteBomb_Item") (== _output "SuperBomb_Item") (== _output "Player") (== _output "DestructibleWall")))))

(fn `SpawnExplosionEmitter`
  (params (ExplosionLenght :type "Float (double-precision)") (DirectionIndex :type Integer))
  (bind _returnvalue (`GameplayStatics.SpawnEmitterAttached` "/Game/MyParticleSystems/Beam/P_Beam.P_Beam" (`self.StaticMeshComponent`) "None" (`self.K2_GetActorLocation`) (`KismetMathLibrary.MakeRotator` 0.0 0.0 (`KismetMathLibrary.RadiansToDegrees` (/ (`KismetMathLibrary.MultiplyByPi` (`KismetMathLibrary.Conv_IntToDouble` DirectionIndex)) 2.0))) "KeepWorldPosition"))
  (`ParticleSystemComponent.SetVectorParameter` _returnvalue "TargetLocation" (`KismetMathLibrary.MakeVector` ExplosionLenght 0.0 (.z (`self.K2_GetActorLocation`)))))

(fn `TraceObstacle`
  (params (DirectionVector :type "Vector Structure"))
  (returns (ExplosionLenght :type "Float (double-precision)"))
  (locals (LastHitLocation :type "Vector Structure"))
  (bind _returnvalue (`self.K2_GetActorLocation`))
  (bind (_outhit _returnvalue_2) (`KismetSystemLibrary.LineTraceSingleForObjects` _returnvalue (+ _returnvalue (* DirectionVector (`self.ExplosionLenght`))) (`|MakeArray` "ObjectTypeQuery2" "ObjectTypeQuery1" :!type "EObjectTypeQuery Enum") false (`|MakeArray` (`self.GetOwner`))))
  (if _returnvalue_2
    (bind _result (`self.IsBlockableObstacle` (`.HitActor` (`GameplayStatics.BreakHitResult` _outhit))))
    (if _result
      (return (`KismetMathLibrary.VSize` (- (`.Location` (`GameplayStatics.BreakHitResult` _outhit)) (`self.K2_GetActorLocation`))))
      (else
        (return (`self.ExplosionLenght`))))
    (else
      (return (`self.ExplosionLenght`)))))

(fn `TraceVictims`
  (params (DirectionVector :type "Vector Structure") (ExplosionLenght :type "Float (double-precision)"))
  (returns (Actors :type "Array of Actor Object Reference"))
  (locals (LastHitLocation :type "Vector Structure") (TraceHits :type "Array of HitResult Structure") (Victims :type "Array of Actor Object Reference"))
  (bind _returnvalue (`self.K2_GetActorLocation`))
  (bind _victims (`local.Victims`))
  (bind (_outhits _returnvalue_2) (`KismetSystemLibrary.LineTraceMultiForObjects` _returnvalue (+ _returnvalue (* DirectionVector ExplosionLenght)) (`|MakeArray` "ObjectTypeQuery2" "ObjectTypeQuery4" :!type "EObjectTypeQuery Enum") false (`|MakeArray` (`self.GetOwner`)) "None" true (struct :`R` 1.0 :`A` 1.0) (struct :`G` 1.0 :`A` 1.0) 10.0))
  (if _returnvalue_2
    (for _array_element _outhits
      (bind (_bblockinghit _binitialoverlap _time _location _impactpoint _normal _impactnormal _physmat _hitactor) (`GameplayStatics.BreakHitResult` _array_element))
      (bind _result (`self.IsVictim` _hitactor))
      (if _result
        (`KismetArrayLibrary.Array_Add` _victims _hitactor)
        (else
          (return))))
    (return _victims)))

(fn `UserConstructionScript`)