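; Character Blueprint for the second player (Player B) in a Bomberman-style game, handling that player's controls.
; PlayerB-specific axis inputs drive the BomberMan move-right and move-forward functions at walk speed, and a hard-bound Right Ctrl key calls the bomb placement event.
; The graph contains only input wiring, with movement and bomb logic defined elsewhere, and the construction script just calls its parent.
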(event `Key|RightControl` :consume false
  (params (Key :type "Key Structure" :default "AnyKey"))
  (:`Pressed`
    (`self.PlaceBomb_Event`)))

(event `InputAxis|PlayerB_MoveRight` :consume false
  (params (AxisValue :type "Float (single-precision)"))
  (`/Game/Blueprints/BomberMan_Movements.BomberMan_MoveRight` AxisValue self (`self.WalkSpeed`)))

(event `InputAxis|PlayerB_MoveForward` :consume false
  (params (AxisValue :type "Float (single-precision)"))
  (`/Game/Blueprints/BomberMan_Movements.BomberMan_MoveForward` AxisValue self (`self.WalkSpeed`)))

(fn `UserConstructionScript`
  (`parent.UserConstructionScript`))